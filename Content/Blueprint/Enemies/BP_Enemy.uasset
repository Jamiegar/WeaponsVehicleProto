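; Enemy AI character that runs a behavior tree and combines health and physical-animation components for combat and ragdoll reactions.
; Perception and incoming damage set the blackboard Player target and the IsFiring flag.
; Ragdoll, stand-up and knockback montage events drive the blackboard State, with a random-duration timer for living ragdolled enemies.
; Death ragdolls it and disables capsule collision, while hover bike overlaps ragdoll, push and damage it.
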(event `self.ReceiveBeginPlay`
  (message `/Game/Blueprint/Interfaces/BPI_Initalizable.Init` (`self.COM_PhysicalAnimation`))
  (message `/Game/Blueprint/Interfaces/BPI_Initalizable.Init` (`self.COM_Health`))
  (`AIController.RunBehaviorTree` (`AIBlueprintHelperLibrary.GetAIController` self) "/Game/Blueprint/Enemies/BehaviourTree/BT_EnemyBehavior.BT_EnemyBehavior"))

(event `self.COM_Health.OnDeath`
  (`/Game/Blueprint/Enemies/COM_PhysicalAnimation.EnterRagdoll` (`self.COM_PhysicalAnimation`))
  (`PrimitiveComponent.SetCollisionEnabled` (`self.CapsuleComponent`) "NoCollision"))

(event `self.COM_PhysicalAnimation.OnEnteredRagdoll`
  (`BlackboardComponent.SetValueAsEnum` (`AIBlueprintHelperLibrary.GetBlackboard` null) "State" (enumliteral `/Game/Blueprint/Enemies/BehaviourTree/E_AIStates` "NewEnumerator3"))
  (if (not (`/Game/Blueprint/Character/Health/COM_Health.IsDead` (`self.COM_Health`)))
    (`KismetSystemLibrary.K2_ClearAndInvalidateTimerHandle` (`self.RagdollTimer`))
    (bind _returnvalue (`KismetSystemLibrary.K2_SetTimerDelegate` (`|CreateDelegate` (`self.COM_PhysicalAnimation`) :!event `StandUp`) (`KismetMathLibrary.RandomFloatInRange` (`self.RagdollDurationMin`) (`self.RagdollDurationMax`))))
    (set `self.RagdollTimer` _returnvalue)
    (else
      (`KismetSystemLibrary.K2_ClearAndInvalidateTimerHandle` (`self.RagdollTimer`)))))

(event `self.AIPerception.OnTargetPerceptionUpdated`
  (params (Actor :type "Actor Object Reference") (Stimulus :type "AIStimulus Structure"))
  (if Stimulus_bSuccessfullySensed
    (bind _asbp_physics_pawn (cast `/Game/Blueprint/Character/BP_PhysicsPawn` Actor)
      (:`then`
        (if (`/Game/Blueprint/Character/Health/COM_Health.IsDead` (`/Game/Blueprint/Character/BP_PhysicsPawn.COM_Health` _asbp_physics_pawn))
          (`BlackboardComponent.SetValueAsObject` (`AIBlueprintHelperLibrary.GetBlackboard` null) "Player" null :!label _label)
          (set `self.isFiring` false)
          (else
            (`BlackboardComponent.SetValueAsObject` (`AIBlueprintHelperLibrary.GetBlackboard` null) "Player" Actor)
            (set `self.isFiring` true))))
      (:`CastFailed`
        (goto _label)))
    (else
      (goto _label))))

(event `self.COM_Health.OnDamageApplied`
  (params (OldHealth :type "Float (double-precision)") (NewHealth :type "Float (double-precision)") (DamagingActor :type "Actor Object Reference"))
  (`BlackboardComponent.SetValueAsObject` (`AIBlueprintHelperLibrary.GetBlackboard` null) "Player" DamagingActor)
  (set `self.isFiring` true))

(event `OnStandUp`
  (`BlackboardComponent.SetValueAsEnum` (`AIBlueprintHelperLibrary.GetBlackboard` null) "State" (enumliteral `/Game/Blueprint/Enemies/BehaviourTree/E_AIStates` "NewEnumerator0")))

(event `/Game/Blueprint/Interfaces/BPI_KnockbackHit.KnockbackHit`
  (`|PlayMontage` (`self.Mesh`) "/Game/Assets/MixamoAnimations/AnimMon_StumbleHit_Montage.AnimMon_StumbleHit_Montage"
    (:`then`
      (`BlackboardComponent.SetValueAsEnum` (`AIBlueprintHelperLibrary.GetBlackboard` null) "State" (enumliteral `/Game/Blueprint/Enemies/BehaviourTree/E_AIStates` "NewEnumerator3")))
    (:`OnNotifyBegin`
      (`BlackboardComponent.SetValueAsEnum` (`AIBlueprintHelperLibrary.GetBlackboard` null) "State" (enumliteral `/Game/Blueprint/Enemies/BehaviourTree/E_AIStates` "NewEnumerator2")))))

(event `self.CapsuleComponent.OnComponentBeginOverlap`
  (params (OverlappedComponent :type "PrimitiveComponent Object Reference") (OtherActor :type "Actor Object Reference") (OtherComp :type "PrimitiveComponent Object Reference") (OtherBodyIndex :type Integer) (bFromSweep :type Boolean) (SweepResult :type "HitResult Structure (by ref)"))
  (cast `/Game/Blueprint/Vehicle/BP_HoverBike` OtherActor)
  (`/Game/Blueprint/Enemies/COM_PhysicalAnimation.EnterRagdoll` (`self.COM_PhysicalAnimation`))
  (`PrimitiveComponent.AddForce` (`self.Mesh`) (* (`self.GetActorForwardVector` OtherActor) (`KismetMathLibrary.VSizeXY` (`self.GetVelocity` OtherActor))) "None" true)
  (`/Game/Blueprint/Character/Health/COM_Health.ApplyDamage` (`self.COM_Health`) 100.0 OtherActor))

(fn `UserConstructionScript`)
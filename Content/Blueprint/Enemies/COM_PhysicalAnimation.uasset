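; Enemy component that drives physical-animation hit reactions, ragdolling and standing up on the owner's skeletal mesh.
; Hits simulate bodies below spine_01 and apply an impulse along the trace, then Tick fades the physics blend weight back out.
; While ragdolled, a downward trace from the pelvis keeps the root component following the body.
; StandUp detects face-up or face-down, aligns root rotation and saves a pose snapshot before ending simulation.
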(event `/Game/Blueprint/Interfaces/BPI_Initalizable.Init`
  (bind _returnvalue (`Actor.GetComponentByClass` (`self.GetOwner`) "/Script/Engine.SkeletalMeshComponent"))
  (bind _returnvalue_2 (`|AddComponentByClass` (`self.GetOwner`) "/Script/Engine.PhysicalAnimationComponent"))
  (bind _output_get (set `self.PhysicalAnimationComp` _returnvalue_2))
  (`PhysicalAnimationComponent.SetSkeletalMeshComponent` _output_get _returnvalue)
  (set `self.SkeletalMesh` _returnvalue)
  (`self.PhysicsSetup`))

(event `Hit`
  (params (Hit :type "HitResult Structure"))
  (bind (_bblockinghit _binitialoverlap _time _distance _location _impactpoint _normal _impactnormal _physmat _hitactor _hitcomponent _hitbonename _bonename _hititem _elementindex _faceindex _tracestart _traceend) (`GameplayStatics.BreakHitResult` Hit))
  (`self.PhysicalAnim`)
  (`PrimitiveComponent.AddImpulse` (`self.SkeletalMesh`) (* (`KismetMathLibrary.Normal` (- _traceend _tracestart)) 10000.0) (select `bool` (== _hitbonename "Pelvis") :`false` _hitbonename :`true` "spine_01") false))

(event `self.ReceiveTick`
  (params (DeltaSeconds :type "Float (single-precision)"))
  (`self.LerpBonesFromPhysicsAnim` DeltaSeconds)
  (`self.UpdateCapsuleLocation`))

(event `PhysicalAnim`
  (if (not (`self.isRagdolling`))
    (set `self.LerpToPosition` true)
    (set `self.HitReactionTimeRemaining` (+ (`self.HitReactionTimeRemaining`) 1.0))
    (`PhysicalAnimationComponent.ApplyPhysicalAnimationProfileBelow` (`self.PhysicalAnimationComp`) "spine_01" (`self.PhysicalAnimProfileName`) false false)
    (`SkeletalMeshComponent.SetAllBodiesBelowSimulatePhysics` (`self.SkeletalMesh`) "spine_01" true false)))

(event `EnterRagdoll`
  (`PhysicalAnimationComponent.ApplyPhysicalAnimationProfileBelow` (`self.PhysicalAnimationComp`) "Pelvis" "Ragdoll" false false)
  (`SkeletalMeshComponent.SetAllBodiesBelowSimulatePhysics` (`self.SkeletalMesh`) "Pelvis" true true)
  (`SkeletalMeshComponent.SetAllBodiesBelowPhysicsBlendWeight` (`self.SkeletalMesh`) "Pelvis" 1.0 false true)
  (set `self.LerpToPosition` false)
  (set `self.isRagdolling` true)
  (`self.OnEnteredRagdoll`))

(event `StandUp`
  (`self.FindCharacterOrientation`)
  (`self.SetCapsuleRotation`)
  (`KismetSystemLibrary.Delay` 0.2)
  (`AnimInstance.SavePoseSnapshot` (`SkeletalMeshComponent.GetAnimInstance` (`self.SkeletalMesh`)) "RagdollPose")
  (`KismetSystemLibrary.Delay` 0.0)
  (`SkeletalMeshComponent.SetAllBodiesSimulatePhysics` (`self.SkeletalMesh`) false)
  (`KismetSystemLibrary.Delay` 0.0)
  (set `self.isRagdolling` false))

(fn `FindCharacterOrientation`
  (bind (_returnvalue_x _returnvalue_y _returnvalue_z) (`KismetMathLibrary.BreakVector` (* (`KismetMathLibrary.GetRightVector` (`SceneComponent.GetSocketRotation` (`self.SkeletalMesh`) "Pelvis")) -1.0)))
  (bind _returnvalue (> _returnvalue_z 0.0))
  (`KismetSystemLibrary.PrintString` (`KismetStringLibrary.Concat_StrStr` "OnBack: " (`KismetStringLibrary.Conv_BoolToString` _returnvalue)))
  (set `self.OnBack` _returnvalue))

(fn `LerpBonesFromPhysicsAnim`
  (params (DeltaTime :type "Float (single-precision)"))
  (if (`self.LerpToPosition`)
    (bind _output_get (set `self.HitReactionTimeRemaining` (- (`KismetMathLibrary.FInterpTo` (`self.HitReactionTimeRemaining`) 0.0 DeltaTime 3.0) (* DeltaTime 0.1))))
    (if (<= _output_get 0.0)
      (set `self.HitReactionTimeRemaining` 0.0)
      (`SkeletalMeshComponent.SetAllBodiesBelowSimulatePhysics` (`self.SkeletalMesh`) "spine_01" false false)
      (set `self.LerpToPosition` false)
      (else
        (`SkeletalMeshComponent.SetAllBodiesBelowPhysicsBlendWeight` (`self.SkeletalMesh`) "spine_01" (`KismetMathLibrary.FMin` (`self.HitReactionTimeRemaining`) 1.0) false true)))))

(fn `PhysicsSetup`
  (set `self.MeshPelvisOffset` (`SceneComponent.RelativeLocation` (`self.SkeletalMesh`))))

(fn `SetCapsuleRotation`
  (bind _returnvalue (- (`SceneComponent.GetSocketLocation` (`self.SkeletalMesh`) "neck_01") (`SceneComponent.GetSocketLocation` (`self.SkeletalMesh`) "Pelvis")))
  (`SceneComponent.K2_SetWorldRotation` (`Actor.RootComponent` (`self.GetOwner`)) (`KismetMathLibrary.MakeRotFromZX` (`KismetMathLibrary.Vector_Up`) (`KismetMathLibrary.SelectVector` (* _returnvalue -1.0) _returnvalue (`self.OnBack`))) false false))

(fn `UpdateCapsuleLocation`
  (locals (TargetGroundLocation :type "Vector Structure" :default (0.0 0.0 0.0)))
  (bind _returnvalue (`SceneComponent.GetSocketLocation` (`self.SkeletalMesh`) "Pelvis"))
  (if (`self.isRagdolling`)
    (bind (_outhit _returnvalue_2) (`KismetSystemLibrary.LineTraceSingle` _returnvalue (+ _returnvalue (0.0 0.0 -100.0)) "TraceTypeQuery1"))
    (set `local.TargetGroundLocation` (`KismetMathLibrary.SelectVector` (`.Location` (`GameplayStatics.BreakHitResult` _outhit)) (`SceneComponent.GetSocketLocation` (`self.SkeletalMesh`) "Pelvis") _returnvalue_2))
    (`SceneComponent.K2_SetWorldLocation` (`Actor.RootComponent` (`self.GetOwner`)) (- (`local.TargetGroundLocation`) (`self.MeshPelvisOffset`)) false false)))
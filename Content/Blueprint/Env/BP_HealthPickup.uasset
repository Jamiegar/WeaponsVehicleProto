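; BP_HealthPickup is a pickup actor that restores health to a BP_PhysicsPawn on contact.
; An overlap on its Sphere casts the other actor to BP_PhysicsPawn and passes HealthIncreaseAmount to that pawn's COMHealth component.
; It then plays the MS_AddedHealth sound at its location, attaches the NS_HealthAdded Niagara effect to the pawn's root, and destroys itself.
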(event `self.Sphere.OnComponentBeginOverlap`
  (params (OverlappedComponent :type "PrimitiveComponent Object Reference") (OtherActor :type "Actor Object Reference") (OtherComp :type "PrimitiveComponent Object Reference") (OtherBodyIndex :type Integer) (bFromSweep :type Boolean) (SweepResult :type "HitResult Structure (by ref)"))
  (bind _asbp_physics_pawn (cast `/Game/Blueprint/Character/BP_PhysicsPawn` OtherActor))
  (`/Game/Blueprint/Character/Health/COM_Health.ApplyHealth` (`/Game/Blueprint/Character/BP_PhysicsPawn.COM_Health` _asbp_physics_pawn) (`self.HealthIncreaseAmount`))
  (`GameplayStatics.SpawnSoundAtLocation` "/Game/Blueprint/Env/Audio/MS_AddedHealth.MS_AddedHealth" (`self.K2_GetActorLocation`) (struct) 1.0 1.0 0.0 null null)
  (`NiagaraFunctionLibrary.SpawnSystemAttached` "/Game/Blueprint/VFX/Systems/NS_HealthAdded.NS_HealthAdded" (`Actor.RootComponent` _asbp_physics_pawn) "None" (250.0 0.0 0.0) (struct :`Yaw` 90.0) "KeepRelativeOffset")
  (`self.K2_DestroyActor`))

(fn `UserConstructionScript`
  (`parent.UserConstructionScript`))
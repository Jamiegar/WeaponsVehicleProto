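; BP_Catapult is an environment catapult that swings when its Hit event is called, then returns to rest.
; Hit enables physics on the Catapult component, changes the PhysicsConstraint's angular orientation target to a raised pitch and wakes the body.
; A one-shot timer of ResetTimer length then calls RestCatapult, which zeroes the target and wakes the body again, so the motion is constraint-driven rather than animated.
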(event `/Game/Blueprint/Interfaces/BPI_Hitable.Hit`
  (params (HitResult :type "HitResult Structure"))
  (`PrimitiveComponent.SetSimulatePhysics` (`self.Catapult`) true)
  (`PhysicsConstraintComponent.SetAngularOrientationTarget` (`self.PhysicsConstraint`) (`KismetMathLibrary.MakeRotator` 0.0 105.0))
  (`PrimitiveComponent.WakeRigidBody` (`self.Catapult`) "None")
  (`KismetSystemLibrary.K2_SetTimerDelegate` (delegate `RestCatapult`) (`self.ResetTimer`)))

(event `RestCatapult`
  (`PhysicsConstraintComponent.SetAngularOrientationTarget` (`self.PhysicsConstraint`) (`KismetMathLibrary.MakeRotator` 0.0 0.0))
  (`PrimitiveComponent.WakeRigidBody` (`self.Catapult`) "None"))

(fn `UserConstructionScript`)
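; Health component that tracks health, applies damage and healing, and signals death.
; Health starts at the default value on Init, and that default also caps healing in ApplyHealth.
; ApplyDamage clamps Health at zero and calls OnDeath before zeroing it, with no guard against repeat calls on later hits.
; Both functions return the updated Health.
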(event `/Game/Blueprint/Interfaces/BPI_Initalizable.Init`
  (set `self.Health` (`self.DefautHealth`)))

(fn `ApplyDamage`
  (params (TakenDamage :type "Float (double-precision)"))
  (returns (NewHealth :type "Float (double-precision)"))
  (bind _returnvalue (- (`self.Health`) TakenDamage))
  (if (<= _returnvalue 0.0)
    (`self.OnDeath`)
    (set `self.Health` 0.0)
    (else
      (set `self.Health` _returnvalue)))
  (return (`self.Health`)))

(fn `ApplyHealth`
  (params (HealthIncrease :type "Float (double-precision)"))
  (returns (NewHealth :type "Float (double-precision)"))
  (bind _returnvalue (+ HealthIncrease (`self.Health`)))
  (if (> _returnvalue (`self.DefautHealth`))
    (set `self.Health` (`self.DefautHealth`))
    (else
      (set `self.Health` _returnvalue)))
  (return (`self.Health`)))
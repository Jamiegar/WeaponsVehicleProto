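; BP_PhysicsController is the player controller for the physics pawn, handling game UI, pausing and input-device tracking.
; On BeginPlay it caches the game instance, adds the menu input mapping, pre-creates the pause widget and starts forest ambience.
; First possession creates the master HUD with the pawn and calls its InitMessage.
; IA_Pause toggles pause, cursor and input mode, while any key press records gamepad use in the game instance.
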(event `self.ReceiveBeginPlay`
  (bind _asbp_weapon_vehicle_instance (cast `/Game/Blueprint/GameInstance/BP_WeaponVehicleInstance` (`GameplayStatics.GetGameInstance`)))
  (set `self.GameInstance` _asbp_weapon_vehicle_instance)
  (`EnhancedInputSubsystemInterface.AddMappingContext` (subsystem `EnhancedInputLocalPlayerSubsystem`) "/Game/Blueprint/Character/Input/Menu/IMC_Menu.IMC_Menu" 0 (struct))
  (bind _returnvalue (`|CreateWidget` "/Game/Blueprint/UI/Menu/UI_Pause.UI_Pause_C"))
  (set `self.PauseMenu` _returnvalue)
  (`GameplayStatics.PlaySound2D` "/Game/Assets/Ultimate_SFX/Ultimate_Animal_Sound_HD_Remake/Cues/Forest_With_Animals_Ambiance_Cue.Forest_With_Animals_Ambiance_Cue" 0.5 1.0 0.0 null null))

(event `Key|AnyKey` :consume false :overrideparent false
  (params (Key :type "Key Structure"))
  (:`Pressed`
    (set `/Game/Blueprint/GameInstance/BP_WeaponVehicleInstance.IsUsingGamepad` (`KismetInputLibrary.Key_IsGamepadKey` Key) (`self.GameInstance`))))

(event `self.ReceivePossess`
  (params (PossessedPawn :type "Pawn Object Reference"))
  (`self.MasterUI`
    (:`then`)
    (:`else`
      (`self.CreateMasterUI`)
      (message `/Game/Blueprint/Interfaces/BPI_Initalizable.Init` PossessedPawn))))

(event `EnhancedInput|/Game/Blueprint/Character/Input/Menu/Actions/IA_Pause`
  (params (ActionValue :type Boolean) (ElapsedSeconds :type "Float (double-precision)") (TriggeredSeconds :type "Float (double-precision)") (InputAction :type "InputAction Object Reference" :default "/Game/Blueprint/Character/Input/Menu/Actions/IA_Pause.IA_Pause"))
  (:`Started`
    (`self.TogglePause`)))

(event `TogglePause`
  (if (`GameplayStatics.IsGamePaused`)
    (`GameplayStatics.SetGamePaused` false)
    (set `self.bShowMouseCursor` false)
    (`WidgetBlueprintLibrary.SetInputMode_GameOnly` self)
    (`Widget.RemoveFromParent` (`self.PauseMenu`))
    (else
      (`GameplayStatics.SetGamePaused` true)
      (set `self.bShowMouseCursor` true)
      (`WidgetBlueprintLibrary.SetInputMode_GameAndUIEx` self (`self.PauseMenu`))
      (`UserWidget.AddToViewport` (`self.PauseMenu`) 0))))

(fn `CreateMasterUI`
  (bind _returnvalue (`|CreateWidget` "/Game/Blueprint/UI/GameUI/MasterUI/UI_GameMaster.UI_GameMaster_C" self (cast `/Game/Blueprint/Character/BP_PhysicsPawn` (`self.K2_GetPawn`) :!pure true)))
  (bind _output_get (set `self.MasterUI` _returnvalue))
  (`UserWidget.AddToViewport` _output_get 0))

(fn `GetMasterUI`
  (returns (`Return Value` :type "/Game/Blueprint/UI/GameUI/MasterUI/UI_GameMaster Object Reference"))
  (return (`self.MasterUI`)))

(fn `UserConstructionScript`)
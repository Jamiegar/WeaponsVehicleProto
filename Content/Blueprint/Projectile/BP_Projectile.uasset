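; BP_Projectile is a splash-damage style projectile that destroys itself when its sphere component hits something.
; On impact it gathers pawns, physics bodies and dynamic actors within a splash radius, ignoring its instigator, and draws a debug sphere.
; Each gets a hit message, and those with a COM_PhysicalAnimation component enter ragdoll and receive an upward force on their skeletal mesh.
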(event `self.Sphere.OnComponentHit`
  (params (HitComponent :type "PrimitiveComponent Object Reference") (OtherActor :type "Actor Object Reference") (OtherComp :type "PrimitiveComponent Object Reference") (NormalImpulse :type "Vector Structure") (Hit :type "HitResult Structure (by ref)"))
  (bind _outactors (`self.TraceForEnemiesInRadius`))
  (for _array_element _outactors
    (message `/Game/Blueprint/Interfaces/BPI_Hitable.Hit` _array_element Hit)
    (bind _returnvalue (`self.GetComponentByClass` _array_element "/Game/Blueprint/Enemies/COM_PhysicalAnimation.COM_PhysicalAnimation_C"))
    (`/Engine/EditorBlueprintResources/StandardMacros.IsValid` _returnvalue
      (:`Is Valid`
        (`/Game/Blueprint/Enemies/COM_PhysicalAnimation.EnterRagdoll` _returnvalue)
        (`PrimitiveComponent.AddForce` (`/Game/Blueprint/Enemies/COM_PhysicalAnimation.SkeletalMesh` _returnvalue) (* (0.0 0.0 1.0) (`self.HitUpForce`)) "None" false))))
  (`self.K2_DestroyActor`))

(fn `TraceForEnemiesInRadius`
  (returns (OutActors :type "Array of Actor Object Reference"))
  (`KismetSystemLibrary.DrawDebugSphere` (`self.K2_GetActorLocation`) (`self.SplashArea`) 12 (struct :`R` 1.0 :`G` 0.071486 :`B` 0.023718 :`A` 1.0) 5.0 1.0)
  (bind _outactors (`KismetSystemLibrary.SphereOverlapActors` (`self.K2_GetActorLocation`) (`self.SplashArea`) (`|MakeArray` "ObjectTypeQuery3" "ObjectTypeQuery4" "ObjectTypeQuery2" :!type "EObjectTypeQuery Enum") null (`|MakeArray` (`self.ActorInstaniator`))))
  (return _outactors))

(fn `UserConstructionScript`)
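; Movement component for the hover bike that turns thrust and steer input into physics forces and adds the input mapping context on possession.
; Each tick a downward trace gates thrust and yaw torque toward desired speeds and switches damping, adding extra downward force when airborne.
; Steering rolls the visual mesh, while curve-driven component timelines ease turning and lean out on release.
; It also drives engine audio start, shutdown and speed parameters.
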(event `self.ReceiveBeginPlay`
  (bind _asbp_hover_bike (cast `/Game/Blueprint/Vehicle/BP_HoverBike` (`self.GetOwner`) :!pure true))
  (bind _asprimitive_component (cast `PrimitiveComponent` (`Actor.RootComponent` (`self.GetOwner`))))
  (set `self.OwnerBody` _asprimitive_component)
  (set `self.EngineSFX` (`/Game/Blueprint/Vehicle/BP_HoverBike.MS_HoverEngine` _asbp_hover_bike))
  (set `self.VisualBike` (`/Game/Blueprint/Vehicle/BP_HoverBike.SkeletalMesh1` _asbp_hover_bike)))

(event `OnStartHoverEngine`
  (`self.StartHoverEngineSound`))

(event `OnShudownHoverEngine`
  (bind _enginesfx (`self.EngineSFX`)
    (:`then`
      (`AudioParameterControllerInterface.SetTriggerParameter` _enginesfx "ShutDownEngine"))
    (:`else`)))

(event `OnPossessed`
  (params (NewController :type "Controller Object Reference"))
  (bind _asplayer_controller (cast `PlayerController` NewController))
  (bind _returnvalue (pcsubsystem `EnhancedInputLocalPlayerSubsystem` _asplayer_controller))
  (`/Engine/EditorBlueprintResources/StandardMacros.IsValid` _returnvalue
    (:`Is Valid`
      (`EnhancedInputSubsystemInterface.AddMappingContext` _returnvalue "/Game/Blueprint/Vehicle/Input/IMC_HoverVehicle.IMC_HoverVehicle" 0 (struct)))))

(event `OnUnpossessed`
  (params (OldController :type "Controller Object Reference"))
  (bind _asplayer_controller (cast `PlayerController` OldController))
  (bind _returnvalue (pcsubsystem `EnhancedInputLocalPlayerSubsystem` _asplayer_controller))
  (`/Engine/EditorBlueprintResources/StandardMacros.IsValid` _returnvalue
    (:`Is Valid`
      (`EnhancedInputSubsystemInterface.RemoveMappingContext` _returnvalue "/Game/Blueprint/Vehicle/Input/IMC_HoverVehicle.IMC_HoverVehicle" (struct)))))

(event `self.ReceiveTick`
  (params (DeltaSeconds :type "Float (single-precision)"))
  (`self.AngularTick` DeltaSeconds)
  (`self.ResetRotationTick` DeltaSeconds)
  (`self.GroundHoverCheck`)
  (`self.CalcCurrentSpeeds`)
  (`self.ApplyMovementForce`)
  (`self.ApplyDampening `)
  (`self.ApplyEngineSFX`))

(event `EnhancedInput|/Game/Blueprint/Vehicle/Input/InputActions/IA_Thrust`
  (params (ActionValue :type "Float (double-precision)") (ElapsedSeconds :type "Float (double-precision)") (TriggeredSeconds :type "Float (double-precision)") (InputAction :type "InputAction Object Reference" :default "/Game/Blueprint/Vehicle/Input/InputActions/IA_Thrust.IA_Thrust"))
  (:`Triggered`
    (if (`self.CanMove`)
      (set `self.DesiredSpeed` (* ActionValue (`self.MaxLinearSpeed`)))))
  (:`Completed`
    (set `self.DesiredSpeed` 0.0)))

(event `EnhancedInput|/Game/Blueprint/Vehicle/Input/InputActions/IA_Steer`
  (params (ActionValue :type "Float (double-precision)") (ElapsedSeconds :type "Float (double-precision)") (TriggeredSeconds :type "Float (double-precision)") (InputAction :type "InputAction Object Reference" :default "/Game/Blueprint/Vehicle/Input/InputActions/IA_Steer.IA_Steer"))
  (bind (_relativerotation_roll _relativerotation_pitch _relativerotation_yaw) (`KismetMathLibrary.BreakRotator` (`SceneComponent.RelativeRotation` (`self.VisualBike`))))
  (:`Triggered`
    (if (`self.CanMove`)
      (set `self.DesiredAngularSpeed` (* ActionValue (`self.MaxAngularSpeed`)))
      (`self.RotateBikeMesh` ActionValue)))
  (:`Started`
    (goto _label :!via `Stop`))
  (:`Completed`
    (set `self.OnStoppedAngularSpeed` (`self.DesiredAngularSpeed`))
    (`|ExecutionSequence`
      (:`then_0`
        (bind _alpha (`/Game/Blueprint/BPFL/Macro_ComponentTimeLine.ComponentTimeLine` (stale `AngularTick` DeltaTime) "/Game/Blueprint/Vehicle/C_AngularDeacceleration.C_AngularDeacceleration" :!label _label)
          (:`Update`
            (set `self.DesiredAngularSpeed` (`KismetMathLibrary.Lerp` (`self.OnStoppedAngularSpeed`) 0.0 _alpha)))
          (:`Completed`
            (set `self.DesiredAngularSpeed` 0.0))))
      (:`then_1`
        (set `self.StartRotation` (`SceneComponent.RelativeRotation` (`self.VisualBike`)))
        (bind _alpha_2 (`/Game/Blueprint/BPFL/Macro_ComponentTimeLine.ComponentTimeLine` (stale `ResetRotationTick` DeltaTime) "/Game/Blueprint/Vehicle/C_ResetRotation.C_ResetRotation" :!label _label_2)
          (:`Update`
            (`SceneComponent.K2_SetRelativeRotation` (`self.VisualBike`) (`KismetMathLibrary.RLerp` (`self.StartRotation`) (`KismetMathLibrary.MakeRotator` 0.0 _relativerotation_pitch _relativerotation_yaw) _alpha_2 true) false false)))))))

(event `AngularTick`
  (params (DeltaTime :type "Float (double-precision)"))
  (goto _label :!via `Tick`))

(event `ResetRotationTick`
  (params (DeltaTime :type "Float (double-precision)"))
  (goto _label_2 :!via `Tick`))

(fn `ApplyDampening `
  (if (`self.IsHoverGrounded`)
    (`PrimitiveComponent.SetLinearDamping` (`self.OwnerBody`) 3.0)
    (`PrimitiveComponent.SetAngularDamping` (`self.OwnerBody`) 5.0)
    (else
      (`PrimitiveComponent.SetLinearDamping` (`self.OwnerBody`) 0.0)
      (`PrimitiveComponent.SetAngularDamping` (`self.OwnerBody`) 50.0)
      (`PrimitiveComponent.AddForce` (`self.OwnerBody`) (0.0 0.0 -2000.0) "None" true))))

(fn `ApplyEngineSFX`
  (bind _returnvalue (`PrimitiveComponent.GetPhysicsLinearVelocity` (`self.OwnerBody`) "None"))
  (bind _enginesfx (`self.EngineSFX`)
    (:`then`
      (`AudioParameterControllerInterface.SetFloatParameter` _enginesfx "Speed" (`KismetMathLibrary.VSizeXY` _returnvalue)))
    (:`else`)))

(fn `ApplyMovementForce`
  (if (`self.IsHoverGrounded`)
    (`PrimitiveComponent.AddForce` (`self.OwnerBody`) (* (`SceneComponent.GetForwardVector` (`self.OwnerBody`)) (- (* (`self.DesiredSpeed`) 10.0) (`self.CurrentSpeed`))) "None" true)
    (`PrimitiveComponent.AddTorqueInDegrees` (`self.OwnerBody`) (* (`SceneComponent.GetUpVector` (`self.OwnerBody`)) (* (- (`self.DesiredAngularSpeed`) (`self.CurrentAngularSpeed`)) (`self.AngularSpeedToTorqueFactor`))) "None" false)))

(fn `CalcCurrentSpeeds`
  (bind _ownerbody (`self.OwnerBody`))
  (bind _ownerbody_2 (`self.OwnerBody`)
    (:`then`
      (bind _returnvalue (`PrimitiveComponent.GetPhysicsLinearVelocity` _ownerbody_2 "None"))
      (set `self.CurrentSpeed` (`KismetMathLibrary.Dot_VectorVector` _returnvalue (`SceneComponent.GetForwardVector` _ownerbody_2)))
      (set `self.CurrentAngularSpeed` (`KismetMathLibrary.Dot_VectorVector` (`PrimitiveComponent.GetPhysicsAngularVelocityInDegrees` _ownerbody "None") (`SceneComponent.GetUpVector` _ownerbody))))
    (:`else`)))

(fn `DisableMovement`
  (set `self.CanMove` false))

(fn `EnableMovement`
  (set `self.CanMove` true))

(fn `GroundHoverCheck`
  (bind _ownerbody (`self.OwnerBody`))
  (bind _returnvalue (`SceneComponent.K2_GetComponentLocation` _ownerbody))
  (bind (_outhit _returnvalue_2) (`KismetSystemLibrary.LineTraceSingle` :`Start` _returnvalue :`End` (- _returnvalue (* (`SceneComponent.GetUpVector` _ownerbody) 75.0)) :`TraceChannel` "TraceTypeQuery1" :`DrawDebugType` "ForOneFrame"))
  (set `self.GroundHit` _outhit)
  (set `self.IsHoverGrounded` _returnvalue_2))

(fn `RotateBikeMesh`
  (params (InputAxis :type "Float (double-precision)"))
  (bind (_relativerotation_roll _relativerotation_pitch _relativerotation_yaw) (`KismetMathLibrary.BreakRotator` (`SceneComponent.RelativeRotation` (`self.VisualBike`))))
  (`SceneComponent.K2_AddRelativeRotation` (`self.VisualBike`) (`KismetMathLibrary.SelectRotator` (struct :`Roll` 0.5) (struct :`Roll` -0.5) (>= InputAxis 0.1)) false false)
  (`SceneComponent.K2_SetRelativeRotation` (`self.VisualBike`) (`KismetMathLibrary.MakeRotator` (`KismetMathLibrary.FClamp` _relativerotation_roll -20.0 20.0) _relativerotation_pitch _relativerotation_yaw) false false))

(fn `StartHoverEngineSound`
  (bind _enginesfx (`self.EngineSFX`))
  (bind _enginesfx_2 (`self.EngineSFX`)
    (:`then`
      (if (`AudioComponent.IsPlaying` _enginesfx_2)
        (`AudioParameterControllerInterface.SetTriggerParameter` _enginesfx "EngineStart")
        (else
          (`AudioComponent.Play` _enginesfx 0.0))))
    (:`else`)))
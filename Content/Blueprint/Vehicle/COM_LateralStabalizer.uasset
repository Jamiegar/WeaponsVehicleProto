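; Vehicle component that applies a lateral stabilizing force to its owning actor's physics body.
; On BeginPlay it caches the owner's root component as a primitive body.
; Each tick it projects that body's linear velocity onto its right vector and adds a force along that axis, scaled by the sideways speed and SpeedToForceFactor.
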(event `self.ReceiveBeginPlay`
  (bind _asprimitive_component (cast `PrimitiveComponent` (`Actor.RootComponent` (`self.GetOwner`))))
  (set `self.OwnerBody` _asprimitive_component))

(event `self.ReceiveTick`
  (params (DeltaSeconds :type "Float (single-precision)"))
  (bind _ownerbody (`self.OwnerBody`)
    (:`then`
      (bind _returnvalue (`PrimitiveComponent.GetPhysicsLinearVelocity` _ownerbody "None"))
      (bind _result (`/Engine/EditorBlueprintResources/StandardMacros.NegateFloat` (`KismetMathLibrary.Dot_VectorVector` _returnvalue (`SceneComponent.GetRightVector` _ownerbody)))
        (:`  `
          (`PrimitiveComponent.AddForce` (`self.OwnerBody`) (* (* _result (`self.SpeedToForceFactor`)) (`SceneComponent.GetRightVector` (`self.OwnerBody`))) "None" false))))
    (:`else`)))
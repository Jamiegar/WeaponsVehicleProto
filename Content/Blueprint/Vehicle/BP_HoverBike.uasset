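; Rideable physics-simulated hover bike that a BP_PhysicsPawn enters by interacting and leaves with IA_Interact.
; Mounting starts the hover engine, disables rider movement, sets the bike weapon flag from HasWeapon, and blends the camera before possessing the bike.
; Possession drives COMHoverVehicleMovementComponent and toggles four corner thrusters.
; Exiting shuts down the engine, teleports the stored pawn to CharacterSpawnPoint, re-enables its movement, and possesses it after the camera blend.
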(event `self.ReceiveBeginPlay`
  (`PrimitiveComponent.SetSimulatePhysics` (`self.SkeletalMesh`) true))

(event `/Game/Blueprint/Interfaces/BPI_Interactable.OnInteract`
  (params (`Interacted Actor` :type "Actor Object Reference"))
  (`/Game/Blueprint/Vehicle/COM_HoverVehicleMovementComponent.OnStartHoverEngine` (`self.COM_HoverVehicleMovementComponent`))
  (`self.SetBikeWeaponActive` `Interacted Actor`)
  (bind _asbp_physics_pawn (cast `/Game/Blueprint/Character/BP_PhysicsPawn` `Interacted Actor`))
  (set `self.PhysicsPawn` _asbp_physics_pawn)
  (`/Game/Blueprint/Character/COM_Physicsbasedmovement.SetMovementActive` (`/Game/Blueprint/Character/BP_PhysicsPawn.COM_Physicsbasedmovement` _asbp_physics_pawn) false)
  (bind _asplayer_controller (cast `PlayerController` (`self.GetController` _asbp_physics_pawn)))
  (`PlayerController.SetViewTargetWithBlend` _asplayer_controller self 0.75 "VTBlend_EaseInOut" 1.0 false)
  (`KismetSystemLibrary.Delay` 0.75)
  (`Controller.Possess` _asplayer_controller self))

(event `self.ReceivePossessed`
  (params (NewController :type "Controller Object Reference"))
  (`/Game/Blueprint/Vehicle/COM_HoverVehicleMovementComponent.OnPossessed` (`self.COM_HoverVehicleMovementComponent`) NewController)
  (`self.ActivateThrusters`))

(event `self.ReceiveUnpossessed`
  (params (OldController :type "Controller Object Reference"))
  (`/Game/Blueprint/Vehicle/COM_HoverVehicleMovementComponent.OnUnpossessed` (`self.COM_HoverVehicleMovementComponent`) OldController)
  (`self.DeactivateThrusters`))

(event `ActivateThrusters`
  (for _array_element (`|MakeArray` (`self.Hover_BR`) (`self.Hover_BL`) (`self.Hover_FL`) (`self.Hover_FR`))
    (set `/Game/Blueprint/Vehicle/SCOM_HoverThruster.ThrusterActive` true _array_element)))

(event `DeactivateThrusters`
  (for _array_element (`|MakeArray` (`self.Hover_BR`) (`self.Hover_BL`) (`self.Hover_FL`) (`self.Hover_FR`))
    (set `/Game/Blueprint/Vehicle/SCOM_HoverThruster.ThrusterActive` false _array_element)))

(event `EnhancedInput|/Game/Blueprint/Character/Input/Actions/IA_Interact`
  (params (ActionValue :type Boolean) (ElapsedSeconds :type "Float (double-precision)") (TriggeredSeconds :type "Float (double-precision)") (InputAction :type "InputAction Object Reference" :default "/Game/Blueprint/Character/Input/Actions/IA_Interact.IA_Interact"))
  (:`Started`
    (`self.SpawnPhysicsPawn`)
    (`/Game/Blueprint/Vehicle/COM_HoverVehicleMovementComponent.OnShudownHoverEngine` (`self.COM_HoverVehicleMovementComponent`))
    (bind _asplayer_controller (cast `PlayerController` (`self.GetController`)))
    (`PlayerController.SetViewTargetWithBlend` _asplayer_controller (`self.PhysicsPawn`) 0.75 "VTBlend_EaseInOut" 0.75 false)
    (`KismetSystemLibrary.Delay` 0.75)
    (`Controller.Possess` _asplayer_controller (`self.PhysicsPawn`))))

(fn `SetBikeWeaponActive`
  (params (InteractedActor :type "Actor Object Reference"))
  (bind _asbp_physics_pawn (cast `/Game/Blueprint/Character/BP_PhysicsPawn` InteractedActor))
  (set `self.EnableBikeWeapon` (`/Game/Blueprint/Character/BP_PhysicsPawn.HasWeapon` _asbp_physics_pawn)))

(fn `SpawnPhysicsPawn`
  (`self.K2_SetActorTransform` (`self.PhysicsPawn`) (`SceneComponent.K2_GetComponentToWorld` (`self.CharacterSpawnPoint`)) false true)
  (`/Game/Blueprint/Character/COM_Physicsbasedmovement.SetMovementActive` (`/Game/Blueprint/Character/BP_PhysicsPawn.COM_Physicsbasedmovement` (`self.PhysicsPawn`)) true))

(fn `UserConstructionScript`)
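; Vehicle component for a secondary projectile ability with an aimed trajectory preview and cooldown.
; Predicts the arc from the weapon's fire socket along the camera's forward vector using fixed speed and gravity, then draws it with spline meshes created through owner messages.
; Firing spawns BP_Projectile along the camera direction with shake and sound, then clears the preview.
; A looping timer fills the UI cooldown and re-enables firing with a sound cue.
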(event `/Game/Blueprint/Interfaces/BPI_Initalizable.Init`
  (set `self.CameraComponent` (`Actor.GetComponentByClass` (`self.GetOwner`) "/Game/Blueprint/Vehicle/COM_VehicleCameraComponent.COM_VehicleCameraComponent_C"))
  (set `self.WeaponComponent` (`Actor.GetComponentByClass` (`self.GetOwner`) "/Game/Blueprint/Weapon/BP_Weapon_Component.BP_Weapon_Component_C")))

(fn `ClearSplinePoints`
  (`SplineComponent.ClearSplinePoints` (`self.Spline`) true)
  (message `/Game/Blueprint/Interfaces/BPI_ProjectilePredict.ClearSplineMeshComponents` (`self.GetOwner`)))

(fn `Cooldown`
  (bind _output_get (set `self.CooldownTime` (+ (`self.CooldownTime`) (`self.Itarator`))))
  (bind _returnvalue (/ _output_get (`self.MaxCooldownTimer`)))
  (`/Game/Blueprint/UI/GameUI/UI_BikeWorldUI.SetCooldown` (`self.GetUI`) _returnvalue)
  (if (>= _returnvalue 1.0)
    (set `self.CanFire` true)
    (`KismetSystemLibrary.K2_ClearAndInvalidateTimerHandle` (`self.CooldownHandle`))
    (`GameplayStatics.SpawnSound2D` "/Game/Assets/Ultimate_SFX/Sci_Fi_Weapon_Sounds/Cues/Weapon_Swap/Weapon_Swap_2_Cue.Weapon_Swap_2_Cue" 1.0 1.0 0.0 null)))

(fn `DrawPath`
  (params (`Predict Params` :type "PredictProjectilePathParams Structure"))
  (`/Engine/EditorBlueprintResources/StandardMacros.IsValid` (`self.Spline`)
    (:`Is Valid`
      (`SplineComponent.ClearSplinePoints` (`self.Spline`) true))
    (:`Is Not Valid`
      (bind _returnvalue (`|AddComponentByClass` :`self` (`self.GetOwner`) :`Class` "/Script/Engine.SplineComponent"))
      (set `self.Spline` _returnvalue)))
  (`self.ClearSplinePoints`)
  (bind _predictresult (`GameplayStatics.Blueprint_PredictProjectilePath_Advanced` (`local.Predict Params`)))
  (for _array_element (`.PathData` (break `PredictProjectilePathResult` _predictresult))
    (`SplineComponent.AddSplinePoint` (`self.Spline`) (`.Location` (break `PredictProjectilePathPointData` _array_element)) "World" true))
  (for _index (range (`SplineComponent.GetNumberOfSplinePoints` (`self.Spline`)))
    (bind _splinmeshcomponent (message `/Game/Blueprint/Interfaces/BPI_ProjectilePredict.AddSplineMeshComponent` (`self.GetOwner`)))
    (bind (_location _tangent) (`SplineComponent.GetLocationAndTangentAtSplinePoint` (`self.Spline`) _index "World"))
    (bind (_location_2 _tangent_2) (`SplineComponent.GetLocationAndTangentAtSplinePoint` (`self.Spline`) (+ _index 1) "World"))
    (`SplineMeshComponent.SetStartAndEnd` _splinmeshcomponent _location _tangent _location_2 _tangent_2 true)))

(fn `FireProjectile`
  (if (`self.CanFire`)
    (bind _returnvalue (`|SpawnActorFromClass` "/Game/Blueprint/Weapon/Projectile/BP_Projectile.BP_Projectile_C" (`SceneComponent.GetSocketTransform` (`self.WeaponComponent`) (`self.ProjectileFirePoint`) "RTS_World") "Undefined" "OverrideRootScale" null null null))
    (bind _projectilemovement (`/Game/Blueprint/Weapon/Projectile/BP_Projectile.ProjectileMovement` _returnvalue))
    (set `MovementComponent.Velocity` (* (`ProjectileMovementComponent.InitialSpeed` _projectilemovement) (`SceneComponent.GetForwardVector` (`/Game/Blueprint/Vehicle/COM_VehicleCameraComponent.VehicleCamera` (`self.CameraComponent`)))) _projectilemovement)
    (`/Game/Blueprint/BPFL/BPFL_Camera.ApplyCameraShake` "/Game/Blueprint/Weapon/CameraShake/BP_WeaponSecondaryFire.BP_WeaponSecondaryFire_C")
    (`GameplayStatics.PlaySoundAtLocation` "/Game/Assets/Ultimate_SFX/Sci_Fi_Weapon_Sounds/Cues/Sci_Fi_Grenade_Launcher/Sci_Fi_Grenade_Launcher_2_Cue.Sci_Fi_Grenade_Launcher_2_Cue" (`SceneComponent.K2_GetComponentLocation` (`self.WeaponComponent`)) (struct) 1.0 1.0 0.0 null null null null)
    (`self.ClearSplinePoints`)
    (`self.StartCooldown`)))

(fn `PredictProjectilePath`
  (if (`self.CanFire`)
    (`self.DrawPath` (make `PredictProjectilePathParams` :`StartLocation` (`SceneComponent.GetSocketLocation` (`self.WeaponComponent`) (`self.ProjectileFirePoint`)) :`LaunchVelocity` (* (`SceneComponent.GetForwardVector` (`/Game/Blueprint/Vehicle/COM_VehicleCameraComponent.VehicleCamera` (`self.CameraComponent`))) 3000.0) :`bTraceWithCollision` true :`ProjectileRadius` 5.0 :`TraceChannel` "ECC_WorldDynamic" :`OverrideGravityZ` -6850.0))))

(fn `StartCooldown`
  (set `self.CanFire` false)
  (set `self.CooldownTime` 0.0)
  (bind _returnvalue (`KismetSystemLibrary.K2_SetTimerDelegate` (`|CreateDelegate` :!event `Cooldown`) (`self.Itarator`) true))
  (set `self.CooldownHandle` _returnvalue))
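; Hover thruster scene component for BP_HoverBike that pushes the bike's skeletal mesh off surfaces below it.
; Each tick while active, it traces down its up axis and applies a spring force at its location from normalized compression.
; Ground contact raises linear and angular damping; a miss clears only linear damping.
; PreviousCompression updates before the return expression reads it, so the spring's velocity damping term evaluates to zero.
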(event `self.ReceiveBeginPlay`
  (bind _asbp_hover_bike (cast `/Game/Blueprint/Vehicle/BP_HoverBike` (`self.GetOwner`)))
  (set `self.HoverBikeOwner` _asbp_hover_bike))

(event `self.ReceiveTick`
  (params (DeltaSeconds :type "Float (single-precision)"))
  (if (`self.ThrusterActive`)
    (`self.HoverBikeOwner`
      (:`then`
        (bind _hoverforce (`self.CalcHoverForce`))
        (`PrimitiveComponent.AddForceAtLocation` (`/Game/Blueprint/Vehicle/BP_HoverBike.SkeletalMesh` (`self.HoverBikeOwner`)) (* (`self.GetUpVector`) _hoverforce) (`self.K2_GetComponentLocation`) "None"))
      (:`else`))))

(fn `CalcHoverForce`
  (returns (HoverForce :type "Float (double-precision)"))
  (locals (Compression :type "Float (double-precision)"))
  (bind _returnvalue (`self.K2_GetComponentLocation`))
  (bind _skeletalmesh (`/Game/Blueprint/Vehicle/BP_HoverBike.SkeletalMesh` (`self.HoverBikeOwner`)))
  (bind (_outhit _returnvalue_2) (`KismetSystemLibrary.LineTraceSingle` _returnvalue (- _returnvalue (* (`self.GetUpVector`) (`self.HoverDistance`))) "TraceTypeQuery1" false (`|MakeArray` (`self.HoverBikeOwner`) :!type "Actor Object Reference") "ForOneFrame"))
  (if _returnvalue_2
    (set `local.Compression` (/ (- (`self.HoverDistance`) (`.Distance` (`GameplayStatics.BreakHitResult` _outhit))) (`self.HoverDistance`)))
    (`PrimitiveComponent.SetLinearDamping` _skeletalmesh 3.0)
    (`PrimitiveComponent.SetAngularDamping` _skeletalmesh 5.0)
    (set `self.PreviousCompression` (`local.Compression`))
    (return (+ (* (/ (- (`local.Compression`) (`self.PreviousCompression`)) (`GameplayStatics.GetWorldDeltaSeconds`)) (`self.Damping`)) (* (`local.Compression`) (`self.HoverStiffness`))))
    (else
      (`PrimitiveComponent.SetLinearDamping` (`/Game/Blueprint/Vehicle/BP_HoverBike.SkeletalMesh` (`self.HoverBikeOwner`)) 0.0))))
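; Vehicle camera component that lets the player look around by yaw and eases the view back to centre afterwards.
; On BeginPlay it finds the owner's camera and stores its starting relative rotation.
; IA_Look adds local yaw from the X axis, closing a gate when input starts and opening it on completion.
; While that gate is open, Tick uses RInterpTo to return the camera to the stored rotation.
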(event `self.ReceiveBeginPlay`
  (bind _output_get (set `self.VehicleCamera` (`Actor.GetComponentByClass` (`self.GetOwner`) "/Script/Engine.CameraComponent")))
  (set `self.ResetCameraRotation` (`SceneComponent.RelativeRotation` _output_get)))

(event `self.ReceiveTick`
  (params (DeltaSeconds :type "Float (single-precision)"))
  (`self.LerpToCameraCentreTick`))

(event `LerpToCameraCentreTick`
  (`/Engine/EditorBlueprintResources/StandardMacros.Gate` true :!label _label
    (:`Exit`
      (`SceneComponent.K2_SetRelativeRotation` (`self.VehicleCamera`) (`KismetMathLibrary.RInterpTo` (`SceneComponent.RelativeRotation` (`self.VehicleCamera`)) (`self.ResetCameraRotation`) (`GameplayStatics.GetWorldDeltaSeconds`) 1.0) false true))))

(event `OpenCameraLerpGate`
  (goto _label :!via `Open`))

(event `CloseCameraLerpGate`
  (goto _label :!via `Close`))

(event `EnhancedInput|/Game/Blueprint/Character/Input/Actions/IA_Look`
  (params (ActionValue :type "Vector2D Structure") (ElapsedSeconds :type "Float (double-precision)") (TriggeredSeconds :type "Float (double-precision)") (InputAction :type "InputAction Object Reference" :default "/Game/Blueprint/Character/Input/Actions/IA_Look.IA_Look"))
  (:`Triggered`
    (`SceneComponent.K2_AddLocalRotation` (`self.VehicleCamera`) (`KismetMathLibrary.MakeRotator` 0.0 0.0 ActionValue_X) false true))
  (:`Started`
    (`self.CloseCameraLerpGate`))
  (:`Completed`
    (`self.OpenCameraLerpGate`)))
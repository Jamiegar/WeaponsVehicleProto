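; BP_ItemMeshComponent is a skeletal mesh component that displays a picked-up item in the hands of a BP_PhysicsPawn.
; On pickup it takes the mesh from the item data and caches the owning pawn.
; It then adds each component class the item requires to the pawn, passing itself, pawn and data before calling InitMessage.
; Finally it snaps to the pawn mesh's GripPoint socket and flags HasWeapon.
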(event `/Game/Blueprint/Interfaces/BPI_Pickup.OnPickup`
  (params (Item :type "/Game/Blueprint/Weapon/WeaponData/DA_Item Object Reference"))
  (set `self.ItemData` Item)
  (bind _itemmesh (`/Game/Blueprint/Weapon/WeaponData/DA_Item.ItemMesh` (`self.ItemData`))
    (:`then`
      (`self.SetSkeletalMeshAsset` _itemmesh)
      (`self.SetOwnerPawn`)
      (`self.AddRequiredComponents`)
      (`self.AttachToOwnerGrip`))
    (:`else`)))

(fn `AddRequiredComponents`
  (bind _itemdata (`self.ItemData`)
    (:`then`
      (for _array_element (`/Game/Blueprint/Weapon/WeaponData/DA_Item.RequireComponents` _itemdata)
        (bind _returnvalue (`|AddComponentByClass` (`self.OwnerPawn`) _array_element (`self.OwnerPawn`) (`self.ItemData`) self))
        (message `/Game/Blueprint/Interfaces/BPI_Initalizable.Init` _returnvalue)))
    (:`else`)))

(fn `AttachToOwnerGrip`
  (`self.K2_AttachToComponent` (`/Game/Blueprint/Character/BP_PhysicsPawn.SkeletalMesh` (`self.OwnerPawn`)) "GripPoint" "SnapToTarget" "SnapToTarget" "SnapToTarget")
  (set `/Game/Blueprint/Character/BP_PhysicsPawn.HasWeapon` true (`self.OwnerPawn`)))

(fn `SetOwnerPawn`
  (bind _asbp_physics_pawn (cast `/Game/Blueprint/Character/BP_PhysicsPawn` (`self.GetOwner`)))
  (set `self.OwnerPawn` _asbp_physics_pawn))
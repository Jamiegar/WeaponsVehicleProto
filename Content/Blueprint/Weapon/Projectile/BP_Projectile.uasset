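; BP_Projectile is an explosive projectile that deals a splash reaction around its point of impact.
; When its sphere hits something, it plays a grenade sound, overlaps actors within SplashArea, excluding its instigator, and sends each a HitMessage.
; Actors with COM_PhysicalAnimation ragdoll and are launched upward by the pelvis, while other physics-simulating roots get an upward impulse.
; It then spawns a dissolve impact Niagara effect and destroys itself.
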(event `self.Sphere.OnComponentHit`
  (params (HitComponent :type "PrimitiveComponent Object Reference") (OtherActor :type "Actor Object Reference") (OtherComp :type "PrimitiveComponent Object Reference") (NormalImpulse :type "Vector Structure") (Hit :type "HitResult Structure (by ref)"))
  (`GameplayStatics.PlaySoundAtLocation` "/Game/Assets/Ultimate_SFX/Sci_Fi_Weapon_Sounds/Cues/Sci_Fi_Grenade/Sci_Fi_Grenade_2_Cue.Sci_Fi_Grenade_2_Cue" (`self.K2_GetActorLocation`) (struct) 1.0 1.0 0.0 null null null null)
  (bind _outactors (`self.TraceForEnemiesInRadius`))
  (for _array_element _outactors
    (message `/Game/Blueprint/Interfaces/BPI_Hitable.Hit` _array_element Hit)
    (bind _returnvalue (`self.GetComponentByClass` _array_element "/Game/Blueprint/Enemies/COM_PhysicalAnimation.COM_PhysicalAnimation_C"))
    (`/Engine/EditorBlueprintResources/StandardMacros.IsValid` _returnvalue
      (:`Is Valid`
        (`/Game/Blueprint/Enemies/COM_PhysicalAnimation.EnterRagdoll` _returnvalue)
        (`PrimitiveComponent.AddImpulse` (`/Game/Blueprint/Enemies/COM_PhysicalAnimation.SkeletalMesh` _returnvalue) (* (0.0 0.0 1.0) (`self.HitUpForce`)) "Pelvis" true))
      (:`Is Not Valid`
        (bind _asprimitive_component (cast `PrimitiveComponent` (`Actor.RootComponent` _array_element) :!pure true))
        (`/Engine/EditorBlueprintResources/StandardMacros.IsValid` _asprimitive_component
          (:`Is Valid`
            (if (`SceneComponent.IsSimulatingPhysics` _asprimitive_component "None")
              (`PrimitiveComponent.AddImpulse` _asprimitive_component (* (0.0 0.0 1.0) 2000.0) "None" true)))))))
  (`NiagaraFunctionLibrary.SpawnSystemAtLocation` "/Game/Blueprint/VFX/Systems/NS_DisolveImpact.NS_DisolveImpact" (`self.K2_GetActorLocation`))
  (`self.K2_DestroyActor`))

(fn `TraceForEnemiesInRadius`
  (returns (OutActors :type "Array of Actor Object Reference"))
  (bind _outactors (`KismetSystemLibrary.SphereOverlapActors` (`self.K2_GetActorLocation`) (`self.SplashArea`) (`|MakeArray` "ObjectTypeQuery3" "ObjectTypeQuery5" "ObjectTypeQuery2" "ObjectTypeQuery4" :!type "EObjectTypeQuery Enum") null (`|MakeArray` (`self.ActorInstaniator`))))
  (return _outactors))

(fn `UserConstructionScript`)